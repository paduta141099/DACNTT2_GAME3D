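; Base enemy character that provides actions for AI: attacking, chasing the player, wielding or sheathing a weapon, and exposing a patrol route.
; Attack plays MM_Jump_Montage and fires OnAttackEnd on completion or interruption, while ChasePlayer uses AIMoveTo toward player 0.
; Wielding spawns BP_Weapon on a hand socket; sheathing starts the same montage, then immediately notifies and destroys the weapon.
; SetMovementSpeed maps walk, jog and sprint states to MaxWalkSpeed.
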(event Custom|Attack
  (Animation|Montage|PlayMontage (Variables|Character|GetMesh) "/Game/Characters/Mannequins/Animations/Manny/MM_Jump_Montage.MM_Jump_Montage"
    (:OnCompleted
      _)
    (:OnInterrupted
      _))
  (Default|CallOnAttackEnd))

(event Custom|ChasePlayer
  (AI|AIMoveTo self "0, 0, 0" (Game|GetPlayerCharacter 0) 5.0 false))

(event Custom|WieldObject
  (bind _returnvalue (Game|SpawnActorfromClass "/Game/A_InteractObjects/BP_Weapon.BP_Weapon_C" (Transformation|GetActorTransform) "Undefined" 0 0))
  (Variables|Default|SetWeapon%20Actor _returnvalue)
  (Transformation|AttachComponentToComponent _returnvalue (Variables|Character|GetMesh) "hand_l_object_socket" "SnapToTarget" "SnapToTarget" "SnapToTarget" true)
  (Variables|Default|SetisWieldingWeapon true))

(event Custom|SheathWeapon
  (Animation|Montage|PlayMontage (Variables|Character|GetMesh) "/Game/Characters/Mannequins/Animations/Manny/MM_Jump_Montage.MM_Jump_Montage"
    (:then
      (Default|CallOnSheathWeapon)
      (Actor|DestroyActor (Variables|Default|GetWeapon%20Actor))
      (Variables|Default|SetisWieldingWeapon false))))

(event EventBeginPlay)

(fn ConstructionScript)

(fn GetPatrolRoute
  (return (Variables|Default|GetPatrolRoute)))

(fn SetMovementSpeed
  (params (Speed :type E_MovementSpeed%20Enum :default "NewEnumerator0"))
  (bind _output_get (Variables|/Script/Engine.CharacterMovementComponent|SetMaxWalkSpeed (Variables|Character|GetCharacterMovement) (Utilities|Select :Index Speed :NewEnumerator0 1e+02 :NewEnumerator1 5e+02 :NewEnumerator2 3.8e+02)))
  (return _output_get))